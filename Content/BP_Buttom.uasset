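; BP_Buttom is a push button pressed by motion controller overlap that fills a progress bar to trigger a video panel.
; Each press animates the button down and back up and adds FillSpeed to Progress, with IsPressed blocking re-entry.
; Tick drains Progress each frame until it reaches full, then calls FillProgressBar on VideoPanel once.
; The progress bar widget receives the button as its Owner.
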(event OnComponentBeginOverlap(ButtomCollision)
  (params (OverlappedComponent :type Primitive%20Component%20Object%20Reference) (OtherActor :type Actor%20Object%20Reference) (OtherComp :type Primitive%20Component%20Object%20Reference) (OtherBodyIndex :type Integer) (bFromSweep :type Boolean) (SweepResult :type Hit%20Result%20Structure%20%28by%20ref%29))
  (bind _buttom (Variables|Default|GetButtom))
  (bind _buttom_2 (Variables|Default|GetButtom))
  (bind _returnvalue (Transformation|GetRelativeTransform _buttom_2))
  (bind _returnvalue_2 (Transformation|GetRelativeTransform _buttom))
  (Utilities|Casting|CastToBP_MotionController OtherActor)
  ;[0.587 1 0.5431] Filling if buttom pressed
  (if (not (Variables|Default|GetIsPressed?))
    (Variables|Default|SetProgress (+ (Variables|Default|GetProgress) (Variables|Default|GetFillSpeed)))
    ;[0.5517 1 0.5386] Press buttom
    (Variables|Default|SetIsPressed? true)
    (Components|MoveComponentTo _buttom_2 (- (.location _returnvalue) "0.000000, 0,4.000000") (.rotation _returnvalue) false false 0.05 false)
    ;[1 0.3199 0.28] Release buttom
    (Components|MoveComponentTo _buttom (+ (.location _returnvalue_2) "0, 0,4.000000") (.rotation _returnvalue_2) false false 0.05 false)
    (Variables|Default|SetIsPressed? false)))

(event EventBeginPlay
  ;[1 1 1] Widget
  (bind _aswbp_progress_bar (Utilities|Casting|CastToWBP_ProgressBar (UserInterface|GetUserWidgetObject (Variables|Default|GetProgressBar))))
  (Variables|/Game/WBP_ProgressBar.WBP_ProgressBar_C|SetOwner _aswbp_progress_bar self))

(event EventTick
  (params (DeltaSeconds :type Float%20%28single-precision%29))
  ;[1 0.8886 0.3571] Is it fill?
  (if (>= (Variables|Default|GetProgress) 1.0)
    ;[0.403 0.5311 1] Play Video
    (Utilities|FlowControl|DoOnce false
      (:Completed
        (Default|FillProgressBar (Variables|Default|GetVideoPanel))))
    (else
      ;[1 0.4678 0.4977] Empty if there is anything
      (if (> (Variables|Default|GetProgress) 0.0)
        (Variables|Default|SetProgress (- (Variables|Default|GetProgress) (Variables|Default|GetEmptySpeed)))))))

(event Input|KeyboardEvents|1
  (params (Key :type Key%20Structure :default "None"))
  ;[0.2292 0.2292 0.2292] Test with keyboard
)

(fn ConstructionScript)